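; BP_CarrotBossHand is a carrot boss hand that becomes vulnerable to the player's spear once three collectibles are picked up.
; Tick watches the player's count, then once changes the Hitable material and sets ChildActor's class to BP_CarrotBossHand.
; A SpearActor overlap with the player nearby swaps that child to BossMesh and hides the hand.
; The hit also spawns BP_BossEnder, plays audio and stops the player's music.
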(event `self.ReceiveBeginPlay`
  (bind _returnvalue (`GameplayStatics.GetActorOfClass` "/Game/SpearSaga/Blueprints/BP_SpearCharacter.BP_SpearCharacter_C"))
  (set `self.Player` _returnvalue)
  (`GameplayStatics.GetAllActorsOfClass` "/Game/SpearSaga/Blueprints/BP_BabyCarrot.BP_BabyCarrot_C"))

(event `self.ReceiveTick`
  (params (DeltaSeconds :type "Float (single-precision)"))
  (if (== (`SpearCharacter.CollectiblesPickedUp` (`self.Player`)) 3)
    (`/Engine/EditorBlueprintResources/StandardMacros.DoOnce` false
      (:`Completed`
        (`PrimitiveComponent.SetMaterial` (`self.Hitable`) 0 "/Game/SpearSaga/Surfaces/Carrot/caroottex_Mat_2.caroottex_Mat_2")
        (`ChildActorComponent.SetChildActorClass` (`self.ChildActor`) "BP_CarrotBossHand_C")))))

(event `self.Hitable.OnComponentBeginOverlap`
  (params (OverlappedComponent :type "PrimitiveComponent Object Reference") (OtherActor :type "Actor Object Reference") (OtherComp :type "PrimitiveComponent Object Reference") (OtherBodyIndex :type Integer) (bFromSweep :type Boolean) (SweepResult :type "HitResult Structure (by ref)"))
  (bind _skeletalmesh (`self.SkeletalMesh`))
  (bind _justafist (`self.JustAFist`))
  (bind _hitable (`self.Hitable`))
  (if (== (`SpearCharacter.CollectiblesPickedUp` (`self.Player`)) 3)
    (if (< (`self.GetDistanceTo` (`self.Player`)) 1300.0)
      (cast `SpearActor` OtherActor)
      (`/Engine/EditorBlueprintResources/StandardMacros.DoOnce` false
        (:`Completed`
          (`ChildActorComponent.SetChildActorClass` (`self.ChildActor`) "/Game/SpearSaga/Models/Carrot/BossMesh.BossMesh_C")
          (`PrimitiveComponent.SetCollisionEnabled` _justafist "NoCollision")
          (`SceneComponent.SetHiddenInGame` _justafist true false)
          (`PrimitiveComponent.SetCollisionEnabled` _hitable "NoCollision")
          (`SceneComponent.SetHiddenInGame` _hitable true false)
          (`PrimitiveComponent.SetCollisionEnabled` _skeletalmesh "NoCollision")
          (`SceneComponent.SetHiddenInGame` _skeletalmesh true false)
          (`ChildActorComponent.SetChildActorClass` (`self.ChildActor1`) "/Game/SpearSaga/Blueprints/BP_BossEnder.BP_BossEnder_C")
          (`AudioComponent.Play` (`self.Audio1`) 0.0)
          (`AudioComponent.Stop` (`/Game/SpearSaga/Blueprints/BP_SpearCharacter.Music` (`self.Player`))))))))

(fn `UserConstructionScript`)
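; BP_BossEnder is a hit target that ends the carrot boss fight in SpearSaga.
; When a SpearActor overlaps its Hitable component while the player is within 300 units, it plays a success sound and spawns an explosion at the BP_CarrotBossHand.
; It then destroys that hand, itself and every SpearActor in the level.
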(event `self.ReceiveBeginPlay`
  (bind _returnvalue (`GameplayStatics.GetActorOfClass` "/Game/SpearSaga/Blueprints/BP_SpearCharacter.BP_SpearCharacter_C"))
  (set `self.Player` _returnvalue))

(event `self.Hitable.OnComponentBeginOverlap`
  (params (OverlappedComponent :type "PrimitiveComponent Object Reference") (OtherActor :type "Actor Object Reference") (OtherComp :type "PrimitiveComponent Object Reference") (OtherBodyIndex :type Integer) (bFromSweep :type Boolean) (SweepResult :type "HitResult Structure (by ref)"))
  (if (< (`self.GetDistanceTo` (`self.Player`)) 300.0)
    (cast `SpearActor` OtherActor)
    (`GameplayStatics.SpawnSound2D` "/Engine/EditorSounds/Notifications/CompileSuccess.CompileSuccess" 1.0 1.0 0.0 null)
    (bind _returnvalue (`GameplayStatics.GetActorOfClass` "/Game/SpearSaga/Blueprints/BP_CarrotBossHand.BP_CarrotBossHand_C"))
    (`NiagaraFunctionLibrary.SpawnSystemAtLocation` "/Game/A/Niagra/NS_Explosion.NS_Explosion" (`self.K2_GetActorLocation` _returnvalue))
    (`self.K2_DestroyActor` _returnvalue)
    (`self.K2_DestroyActor`)
    (bind _outactors (`GameplayStatics.GetAllActorsOfClass` "/Script/GMTK2023.SpearActor"))
    (for _array_element _outactors
      (`self.K2_DestroyActor` _array_element))))

(fn `UserConstructionScript`)